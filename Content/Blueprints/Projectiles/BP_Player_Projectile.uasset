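; Player projectile for a side-scroller that damages whatever it hits, then destroys itself.
; The construction script casts the instigator to SideScrollerCharacter and calls InvertBullet, negating the projectile movement's X velocity when that returns true.
; The Hit event applies the Damage variable to the other actor with the projectile as damage causer.
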(event `self.ReceiveHit`
  (params (MyComp :type "PrimitiveComponent Object Reference") (Other :type "Actor Object Reference") (OtherComp :type "PrimitiveComponent Object Reference") (bSelfMoved :type Boolean) (HitLocation :type "Vector Structure") (HitNormal :type "Vector Structure") (NormalImpulse :type "Vector Structure") (Hit :type "HitResult Structure (by ref)"))
  (`GameplayStatics.ApplyDamage` Other (`self.Damage`) null self)
  (`self.K2_DestroyActor`))

(fn `UserConstructionScript`
  (bind _projectilemovement (`self.ProjectileMovement`))
  (bind (_velocity_x _velocity_y _velocity_z) (`KismetMathLibrary.BreakVector` (`MovementComponent.Velocity` _projectilemovement)))
  (bind _asside_scroller_character (cast `/Game/Blueprints/SideScrollerCharacter` (`self.GetInstigator`)))
  (bind _newparam (`/Game/Blueprints/SideScrollerCharacter.InvertBullet` _asside_scroller_character))
  (if _newparam
    (set `MovementComponent.Velocity` (`KismetMathLibrary.MakeVector` (* _velocity_x -1.0) _velocity_y _velocity_z) _projectilemovement)))