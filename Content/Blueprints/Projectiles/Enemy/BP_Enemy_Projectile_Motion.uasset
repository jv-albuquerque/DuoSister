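; Enemy projectile that lobs itself in a high ballistic arc toward the player's position at spawn.
; On BeginPlay it solves the trajectory equation for a fixed 75-degree launch, using Y distance, offset-adjusted height difference and projectile gravity.
; The result sets the ProjectileMovement speeds and a velocity in the YZ plane, with no later homing.
; The square root keeps Y velocity non-negative, and SetVelocity is an empty stub.
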(event `self.ReceiveBeginPlay`
  (bind (_returnvalue_x _returnvalue_y _returnvalue_z) (`KismetMathLibrary.BreakVector` (`self.K2_GetActorLocation`)))
  (bind (_returnvalue_x_2 _returnvalue_y_2) (`KismetMathLibrary.BreakVector` (`self.K2_GetActorLocation`)))
  (bind _distance (`self.Distance`))
  (bind _projectilemovement (`self.ProjectileMovement`))
  (bind (_returnvalue_x_3 _returnvalue_y_3) (`KismetMathLibrary.BreakVector` (`self.K2_GetActorLocation` (`GameplayStatics.GetPlayerCharacter` 0))))
  (bind (_returnvalue_x_4 _returnvalue_y_4 _returnvalue_z_2) (`KismetMathLibrary.BreakVector` (`self.K2_GetActorLocation` (`GameplayStatics.GetPlayerCharacter` 0))))
  ;[1 1 1] Set Sine and Cossine of 75
  (set `self.CosAlpha` 0.258819)
  (set `self.SenAlpha` 0.965926)
  ;[1 1 1] Distance between the player and the projectile, ignoring the height
  (set `self.Distance` (- _returnvalue_y_3 _returnvalue_y_2))
  ;[1 1 1] Tan of 75
  (set `self.TanAlpha` 3.73205)
  ;[1 1 1] Set hight between player and the projectile
  (set `self.Height` (- (+ _returnvalue_z_2 (`self.Offset`)) _returnvalue_z))
  ;[1 1 1] Velocity in the Y axis = sqrt ( g * d^2 / 2 ( h - d * tanA))
  (set `self.VelocityY` (`KismetMathLibrary.Sqrt` (/ (* (`MovementComponent.GetGravityZ` (`self.ProjectileMovement`)) _distance _distance) (* 2.0 (- (`self.Height`) (* (`self.Distance`) (`self.TanAlpha`)))))))
  ;[1 1 1] Velocity in the Z axis = Voy * tanA
  (set `self.VelocityZ` (* (`self.VelocityY`) (`self.TanAlpha`)))
  (bind _output_get (set `ProjectileMovementComponent.MaxSpeed` (/ (`self.VelocityY`) (`self.CosAlpha`)) _projectilemovement))
  (set `ProjectileMovementComponent.InitialSpeed` _output_get _projectilemovement)
  (set `MovementComponent.Velocity` (`KismetMathLibrary.MakeVector` 0.0 (`self.VelocityY`) (`self.VelocityZ`)) _projectilemovement))

(fn `SetVelocity`
  (params (NewVelocity :type "Float (double-precision)")))

(fn `UserConstructionScript`
  (`parent.UserConstructionScript`))