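; Player projectile for a side-scroller that damages enemies it overlaps.
; The construction script asks the instigating SideScrollerCharacter whether to invert the bullet and, if so, flips the projectile movement's X velocity.
; A sphere overlap applies damage to BP_Enemy actors, then destroys the projectile whatever it touched; a Hit event also destroys it.
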(event `self.ReceiveHit`
  (params (MyComp :type "PrimitiveComponent Object Reference") (Other :type "Actor Object Reference") (OtherComp :type "PrimitiveComponent Object Reference") (bSelfMoved :type Boolean) (HitLocation :type "Vector Structure") (HitNormal :type "Vector Structure") (NormalImpulse :type "Vector Structure") (Hit :type "HitResult Structure (by ref)"))
  (`self.K2_DestroyActor`))

(event `self.SphereCollision.OnComponentBeginOverlap`
  (params (OverlappedComponent :type "PrimitiveComponent Object Reference") (OtherActor :type "Actor Object Reference") (OtherComp :type "PrimitiveComponent Object Reference") (OtherBodyIndex :type Integer) (bFromSweep :type Boolean) (SweepResult :type "HitResult Structure (by ref)"))
  (bind _asbp_enemy (cast `/Game/Blueprints/Enemys/BP_Enemy` OtherActor)
    (:`then`
      (`GameplayStatics.ApplyDamage` _asbp_enemy (`self.Damage`) null self))
    (:`CastFailed`
      _))
  (`self.K2_DestroyActor`))

(fn `UserConstructionScript`
  (bind _projectilemovement (`self.ProjectileMovement`))
  (bind (_velocity_x _velocity_y _velocity_z) (`KismetMathLibrary.BreakVector` (`MovementComponent.Velocity` _projectilemovement)))
  (bind _asside_scroller_character (cast `/Game/Blueprints/SideScrollerCharacter` (`self.GetInstigator`)))
  (bind _newparam (`/Game/Blueprints/SideScrollerCharacter.InvertBullet` _asside_scroller_character))
  (if _newparam
    (set `MovementComponent.Velocity` (`KismetMathLibrary.MakeVector` (* _velocity_x -1.0) _velocity_y _velocity_z) _projectilemovement)))