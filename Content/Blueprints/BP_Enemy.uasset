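; BP_Enemy is an enemy for a side-scroller that hurts the player on contact and can be killed.
; A capsule overlap with a SideScrollerCharacter applies the enemy's Damage to that character.
; Health starts at MaxHealth on BeginPlay and drops with any damage received, printing the remaining value and destroying the actor at zero or below.
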(event `self.ReceiveBeginPlay`
  (set `self.CurrentHealth` (`self.MaxHealth`)))

(event `self.CapsuleComponent.OnComponentBeginOverlap`
  (params (OverlappedComponent :type "PrimitiveComponent Object Reference") (OtherActor :type "Actor Object Reference") (OtherComp :type "PrimitiveComponent Object Reference") (OtherBodyIndex :type Integer) (bFromSweep :type Boolean) (SweepResult :type "HitResult Structure (by ref)"))
  (bind _asside_scroller_character (cast `/Game/SideScrollerBP/Blueprints/SideScrollerCharacter` OtherActor))
  (`GameplayStatics.ApplyDamage` _asside_scroller_character (`self.Damage`)))

(event `self.ReceiveAnyDamage`
  (params (Damage :type "Float (single-precision)") (DamageType :type "DamageType Object Reference") (InstigatedBy :type "Controller Object Reference") (DamageCauser :type "Actor Object Reference"))
  (set `self.CurrentHealth` (- (`self.CurrentHealth`) Damage))
  (`KismetSystemLibrary.PrintString` (`KismetStringLibrary.Concat_StrStr` "Enemy Health" (`KismetStringLibrary.Conv_DoubleToString` (`self.CurrentHealth`))))
  (if (<= (`self.CurrentHealth`) 0.0)
    (`self.K2_DestroyActor`)))

(fn `UserConstructionScript`)