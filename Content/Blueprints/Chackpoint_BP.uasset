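; Checkpoint actor that sets the player's respawn point when the player first touches it.
; On BeginPlay it finds the actor tagged GameController and caches it as a GameController reference.
; When the player character overlaps its Box, it passes its own location to that controller's SetRespawnPoint, then sets AlreadyTaken so it fires only once.
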(event `self.ReceiveBeginPlay`
  (bind _outactors (`GameplayStatics.GetAllActorsWithTag` "GameController"))
  (bind _asgame_controller (cast `/Game/Blueprints/GameController` (`|GetArrayItem` _outactors)))
  (set `self.GameController` _asgame_controller))

(event `self.Box.OnComponentBeginOverlap`
  (params (OverlappedComponent :type "PrimitiveComponent Object Reference") (OtherActor :type "Actor Object Reference") (OtherComp :type "PrimitiveComponent Object Reference") (OtherBodyIndex :type Integer) (bFromSweep :type Boolean) (SweepResult :type "HitResult Structure (by ref)"))
  (if (and (== OtherActor (`GameplayStatics.GetPlayerCharacter` 0)) (not (`self.AlreadyTaken`)))
    (`/Game/Blueprints/GameController.SetRespawnPoint` (`self.GameController`) (`self.K2_GetActorLocation`))
    (set `self.AlreadyTaken` true)))

(fn `UserConstructionScript`)