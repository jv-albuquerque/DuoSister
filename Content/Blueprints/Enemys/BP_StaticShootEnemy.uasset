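; BP_StaticShootEnemy is an enemy that fires BP_Enemy_Projectile_One along its facing direction, with no movement or aiming logic in this file.
; From BeginPlay, TryShoot re-runs itself on a short Delay, checking player distance and CanShoot before calling Shoot.
; Shoot records the shot time and spawns the projectile with itself as Instigator, using LocalToShoot for a transform ahead of and above the actor.
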(event `self.ReceiveBeginPlay`
  (`parent.ReceiveBeginPlay`)
  (`self.TryShoot`))

(event `Shoot`
  ;[1 1 1] Event to shoot the projectile
  (set `self.TimeLastShoot` (`GameplayStatics.GetTimeSeconds`))
  (bind _position (`self.LocalToShoot` (1.0 0.5 0.5)))
  (`|SpawnActorFromClass` "/Game/Blueprints/Projectiles/Enemy/BP_Enemy_Projectile_One.BP_Enemy_Projectile_One_C" _position "Undefined" "OverrideRootScale" null self))

(event `TryShoot`
  ;[1 1 1] Event that try to shoot
  (if (and (<= (`KismetMathLibrary.Vector_Distance` (`self.K2_GetActorLocation` (`GameplayStatics.GetPlayerCharacter` 0)) (`self.K2_GetActorLocation`)) 3000.0) (`self.CanShoot`))
    (`self.Shoot`))
  (`KismetSystemLibrary.Delay` 0.25)
  (`self.TryShoot`))

(fn `LocalToShoot`
  (params (Scale :type "Vector Structure"))
  (returns (Position :type "Transform Structure"))
  (bind (_returnvalue_x _returnvalue_y _returnvalue_z) (`KismetMathLibrary.BreakVector` (+ (`self.K2_GetActorLocation`) (* (`self.GetActorForwardVector`) 80.0))))
  (return (`KismetMathLibrary.MakeTransform` (`KismetMathLibrary.MakeVector` _returnvalue_x _returnvalue_y (+ _returnvalue_z 40.0)) (`self.K2_GetActorRotation`) Scale)))

(fn `UserConstructionScript`
  (`parent.UserConstructionScript`))