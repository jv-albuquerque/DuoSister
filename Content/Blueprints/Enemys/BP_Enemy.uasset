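; BP_Enemy is an enemy for a side-scroller that patrols, deals contact damage and is destroyed when its health runs out.
; When movement is enabled, MoveTo loops AI moves through the PointA list, reissuing on a timer from each request rather than on arrival.
; Capsule overlap damages the player, then briefly toggles a collision channel to Ignore so lingering contact hits again.
; Overlapping any TriggerBox makes it jump.
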(event `self.ReceiveBeginPlay`
  (set `CharacterMovementComponent.JumpZVelocity` (`self.JumpForce`) (`self.CharacterMovement`))
  (set `self.CurrentHealth` (`self.MaxHealth`))
  (if (`self.Move`)
    (`self.MoveTo`)))

(event `self.ReceiveAnyDamage`
  (params (Damage :type "Float (single-precision)") (DamageType :type "DamageType Object Reference") (InstigatedBy :type "Controller Object Reference") (DamageCauser :type "Actor Object Reference"))
  ;[1 1 1] Recive damage
  (set `self.CurrentHealth` (- (`self.CurrentHealth`) Damage))
  (if (<= (`self.CurrentHealth`) 0.0)
    (`self.K2_DestroyActor`)))

(event `self.CapsuleComponent.OnComponentBeginOverlap`
  (params (OverlappedComponent :type "PrimitiveComponent Object Reference") (OtherActor :type "Actor Object Reference") (OtherComp :type "PrimitiveComponent Object Reference") (OtherBodyIndex :type Integer) (bFromSweep :type Boolean) (SweepResult :type "HitResult Structure (by ref)"))
  ;[1 1 1] Deal damage by the body in the player
  (bind _asside_scroller_character (cast `/Game/Blueprints/SideScrollerCharacter` OtherActor))
  (`GameplayStatics.ApplyDamage` _asside_scroller_character (`self.Damage`))
  ;[1 1 1] to make the player be hitten again even if he still inside de enemy
  (`PrimitiveComponent.SetCollisionResponseToChannel` (`self.CapsuleComponent`) "ECC_GameTraceChannel2" "ECR_Ignore")
  (`KismetSystemLibrary.Delay` 0.1)
  (`PrimitiveComponent.SetCollisionResponseToChannel` (`self.CapsuleComponent`) "ECC_GameTraceChannel2" "ECR_Overlap"))

(event `MoveTo`
  ;[1 1 1] Move to a position and has a delay to call it again
  (bind _target_position (`self.SetDestination`))
  (`|AIMoveTo` self _target_position null
    (:`then`
      (`KismetSystemLibrary.Delay` (`self.DelayToMove`))
      (`self.MoveTo`))))

(event `self.ReceiveActorBeginOverlap`
  (params (OtherActor :type "Actor Object Reference"))
  (cast `TriggerBox` OtherActor)
  (`self.Jump`))

(fn `SetDestination`
  (returns (`Target Position` :type "Vector Structure"))
  (`/Engine/EditorBlueprintResources/StandardMacros.IncrementInt` (`self.index`)
    (:`  `
      (if (>= (`self.index`) (`KismetArrayLibrary.Array_Length` (`self.PointA`)))
        (set `self.index` 0))
      (return (`|GetArrayItem` (`self.PointA`) (`self.index`))))))

(fn `UserConstructionScript`)