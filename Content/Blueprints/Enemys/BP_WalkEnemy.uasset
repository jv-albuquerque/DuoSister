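; BP_WalkEnemy is a walking enemy that wanders the navmesh at random.
; On BeginPlay it applies its jump force and starts a movement loop that sends it to a random navigable point nearby, re-rolling after a configurable delay.
; When jumping is enabled, overlapping a TriggerBox makes it jump, so placed triggers act as jump spots.
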(event `self.ReceiveBeginPlay`
  (`parent.ReceiveBeginPlay`)
  (set `CharacterMovementComponent.JumpZVelocity` (`self.JumpForce`) (`self.CharacterMovement`))
  (`self.MoveTo`))

(event `MoveTo`
  ;[1 1 1] Move to a position and has a delay to call it again
  (`self.SetDestination`)
  (`|AIMoveTo` self (`self.Target`) null
    (:`then`
      (`KismetSystemLibrary.Delay` (`self.DelayToMove`))
      (`self.MoveTo`))))

(event `self.ReceiveActorBeginOverlap`
  (params (OtherActor :type "Actor Object Reference"))
  (if (`self.canJump`)
    (cast `TriggerBox` OtherActor)
    (`self.Jump`)))

(fn `SetDestination`
  (set `self.Target` (`NavigationSystemV1.K2_GetRandomLocationInNavigableRadius` (`self.K2_GetActorLocation`) 2000.0 null null))
  (return))

(fn `UserConstructionScript`
  (`parent.UserConstructionScript`))