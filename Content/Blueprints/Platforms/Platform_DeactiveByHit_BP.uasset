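; Side-scroller platform that drops out when the player touches it, then returns.
; Trigger overlap waits, disables actor collision and plays the Rotate timeline to shift the cube in X and pitch it, then reverses and re-enables collision after delays.
; A Deactivater volume makes the cube ignore a custom collision channel while the player overlaps it, allowing jump-through.
; Both behaviors share the Activate flag as a gate.
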(event `self.ReceiveBeginPlay`
  ;[1 1 1] Get the initial position
  (set `self.InitialPosition` (`SceneComponent.K2_GetComponentLocation` (`self.Cube`))))

(event `self.Trigger.OnComponentBeginOverlap`
  (params (OverlappedComponent :type "PrimitiveComponent Object Reference") (OtherActor :type "Actor Object Reference") (OtherComp :type "PrimitiveComponent Object Reference") (OtherBodyIndex :type Integer) (bFromSweep :type Boolean) (SweepResult :type "HitResult Structure (by ref)"))
  ;[1 1 1] Trigger to start fall
  (if (`self.Activate`)
    (cast `/Game/Blueprints/SideScrollerCharacter` OtherActor)
    (`KismetSystemLibrary.Delay` (`self.DelayToDisappear`))
    (set `self.Activate` false)
    (`self.Down`)
    (`self.SetActorEnableCollision` false)
    (`KismetSystemLibrary.Delay` (`self.DelayToAppear`))
    (`self.Up`)
    (`KismetSystemLibrary.Delay` 1.0)
    (set `self.Activate` true)
    (`self.SetActorEnableCollision` true)))

(event `Down`
  ;[1 1 1] Rotation Animation
  (bind (_direction _xposition _rotation) (`Timeline|Rotate` :!via `PlayFromStart` :!label _label)
    (:`Update`
      (`self.SetPosition` _xposition)
      (`self.SetRotation` _rotation))))

(event `Up`
  ;[1 1 1] Rotation Animation
  (goto _label :!via `ReverseFromEnd`))

(event `self.Deactivater.OnComponentBeginOverlap`
  (params (OverlappedComponent :type "PrimitiveComponent Object Reference") (OtherActor :type "Actor Object Reference") (OtherComp :type "PrimitiveComponent Object Reference") (OtherBodyIndex :type Integer) (bFromSweep :type Boolean) (SweepResult :type "HitResult Structure (by ref)"))
  ;[1 1 1] JumpThought
  (if (`self.Activate`)
    (cast `/Game/Blueprints/SideScrollerCharacter` OtherActor)
    (set `self.Activate` false)
    (`PrimitiveComponent.SetCollisionResponseToChannel` (`self.Cube`) "ECC_GameTraceChannel2" "ECR_Ignore")))

(event `self.Deactivater.OnComponentEndOverlap`
  (params (OverlappedComponent :type "PrimitiveComponent Object Reference") (OtherActor :type "Actor Object Reference") (OtherComp :type "PrimitiveComponent Object Reference") (OtherBodyIndex :type Integer))
  ;[1 1 1] JumpThought
  (cast `/Game/Blueprints/SideScrollerCharacter` OtherActor)
  (set `self.Activate` true)
  (`PrimitiveComponent.SetCollisionResponseToChannel` (`self.Cube`) "ECC_GameTraceChannel2" "ECR_Block"))

(fn `UserConstructionScript`)