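; One-way jump-through platform for the side-scroller that toggles its Cube's response on a custom collision channel between Block and Ignore.
; DeactivateChecker ignores that channel while a SideScrollerCharacter overlaps it and restores blocking on exit.
; Checker registers or clears the platform on the overlapping character, supporting drop-down through JumpDown.
; JumpDown briefly ignores the channel, then restores blocking unless the player still overlaps DeactivateChecker.
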(event `self.Checker.OnComponentBeginOverlap`
  (params (OverlappedComponent :type "PrimitiveComponent Object Reference") (OtherActor :type "Actor Object Reference") (OtherComp :type "PrimitiveComponent Object Reference") (OtherBodyIndex :type Integer) (bFromSweep :type Boolean) (SweepResult :type "HitResult Structure (by ref)"))
  ;[1 1 1] Used to jump down the platform
  (bind _asside_scroller_character (cast `/Game/SideScrollerBP/Blueprints/SideScrollerCharacter` OtherActor))
  (`/Game/SideScrollerBP/Blueprints/SideScrollerCharacter.SetPlatform` _asside_scroller_character self))

(event `self.DeactivateChecker.OnComponentBeginOverlap`
  (params (OverlappedComponent :type "PrimitiveComponent Object Reference") (OtherActor :type "Actor Object Reference") (OtherComp :type "PrimitiveComponent Object Reference") (OtherBodyIndex :type Integer) (bFromSweep :type Boolean) (SweepResult :type "HitResult Structure (by ref)"))
  ;[1 1 1] Deactivate the platform
  (cast `/Game/SideScrollerBP/Blueprints/SideScrollerCharacter` OtherActor)
  (if true
    (`PrimitiveComponent.SetCollisionResponseToChannel` (`self.Cube`) "ECC_GameTraceChannel2" "ECR_Ignore")))

(event `self.Checker.OnComponentEndOverlap`
  (params (OverlappedComponent :type "PrimitiveComponent Object Reference") (OtherActor :type "Actor Object Reference") (OtherComp :type "PrimitiveComponent Object Reference") (OtherBodyIndex :type Integer))
  ;[1 1 1] Used to jump down the platform
  (bind _asside_scroller_character (cast `/Game/SideScrollerBP/Blueprints/SideScrollerCharacter` OtherActor))
  (`/Game/SideScrollerBP/Blueprints/SideScrollerCharacter.SetPlatform` _asside_scroller_character null))

(event `self.DeactivateChecker.OnComponentEndOverlap`
  (params (OverlappedComponent :type "PrimitiveComponent Object Reference") (OtherActor :type "Actor Object Reference") (OtherComp :type "PrimitiveComponent Object Reference") (OtherBodyIndex :type Integer))
  ;[1 1 1] Activate the platform
  (cast `/Game/SideScrollerBP/Blueprints/SideScrollerCharacter` OtherActor)
  (`PrimitiveComponent.SetCollisionResponseToChannel` (`self.Cube`) "ECC_GameTraceChannel2" "ECR_Block"))

(event `JumpDown`
  ;[1 1 1] Function to jump down the platform
  (`PrimitiveComponent.SetCollisionResponseToChannel` (`self.Cube`) "ECC_GameTraceChannel2" "ECR_Ignore")
  (`KismetSystemLibrary.Delay` 0.5)
  (if (not (`PrimitiveComponent.IsOverlappingActor` (`self.DeactivateChecker`) (`GameplayStatics.GetPlayerCharacter` 0)))
    (`PrimitiveComponent.SetCollisionResponseToChannel` (`self.Cube`) "ECC_GameTraceChannel2" "ECR_Block")))

(fn `UserConstructionScript`
  ;[1 1 1] Start the platform deactivated
  (`PrimitiveComponent.SetCollisionResponseToChannel` (`self.Cube`) "ECC_GameTraceChannel2" "ECR_Block"))