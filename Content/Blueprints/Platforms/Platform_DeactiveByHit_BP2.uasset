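; Side-scroller platform that drops out of play shortly after the player character overlaps its Checker, then returns after a delay.
; The Rotate timeline slides the Cube along its cached backward vector and pitches it from its initial rotation, reversing to bring it back.
; An Activated flag blocks retriggering during the cycle, and actor collision stays off until one second after the return starts.
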(event `self.ReceiveBeginPlay`
  (set `self.InitialPosition` (`SceneComponent.RelativeLocation` (`self.Cube`)))
  (set `self.BackVector` (* (`SceneComponent.GetForwardVector` (`self.Cube`)) -1.0))
  (set `self.InitialRotation` (`SceneComponent.K2_GetComponentRotation` (`self.Cube`))))

(event `self.Checker.OnComponentBeginOverlap`
  (params (OverlappedComponent :type "PrimitiveComponent Object Reference") (OtherActor :type "Actor Object Reference") (OtherComp :type "PrimitiveComponent Object Reference") (OtherBodyIndex :type Integer) (bFromSweep :type Boolean) (SweepResult :type "HitResult Structure (by ref)"))
  ;[1 1 1] Trigger to start fall, than start go back
  (if (`self.Activated`)
    (cast `/Game/Blueprints/SideScrollerCharacter` OtherActor)
    (`KismetSystemLibrary.Delay` (`self.DelayToDisappear`))
    (set `self.Activated` false)
    (`self.Down`)
    (`self.SetActorEnableCollision` false)
    (`KismetSystemLibrary.Delay` (`self.DelayToAppear`))
    (`self.Up`)
    (`KismetSystemLibrary.Delay` 1.0)
    (set `self.Activated` true)
    (`self.SetActorEnableCollision` true)))

(event `Down`
  (bind (_direction _backposition _rotation) (`Timeline|Rotate` :!via `PlayFromStart` :!label _label)
    (:`Update`
      (`self.SetPosition` _backposition)
      (`self.SetRotation` _rotation))))

(event `Up`
  (goto _label :!via `ReverseFromEnd`))

(fn `UserConstructionScript`
  (`parent.UserConstructionScript`))