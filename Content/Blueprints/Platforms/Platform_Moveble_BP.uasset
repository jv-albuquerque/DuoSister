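; Moving platform actor that cycles endlessly through an array of target locations.
; BeginPlay prints an error if no targets exist, otherwise starts at the NextToGo index, falling back to zero if too high.
; Tick moves it along the normalized direction to the current target by Speed per frame, without delta-time scaling or sweep.
; Within 2 cm of the target, ResetTime advances the index, wrapping to the first.
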(event `self.ReceiveBeginPlay`
  ;[1 1 1] Verify if has some target to go
  (if (<= (`KismetArrayLibrary.Array_Length` (`self.targets`)) 0)
    (`KismetSystemLibrary.PrintString` "Moveble Platform ERRO -- Need to add target locations" true true (struct :`R` 1.0 :`A` 1.0))
    (else
      (`self.Start`))))

(event `self.ReceiveTick`
  (params (DeltaSeconds :type "Float (single-precision)"))
  (bind _returnvalue (- (`|GetArrayItem` (`self.targets`) (`self.index`)) (`self.K2_GetActorLocation`)))
  (if (<= (`KismetMathLibrary.Vector_Distance` (`self.K2_GetActorLocation`) (`|GetArrayItem` (`self.targets`) (`self.index`))) 2.0)
    (`self.ResetTime`))
  (`self.K2_SetActorLocation` (+ (* (/ _returnvalue (`KismetMathLibrary.VSize` _returnvalue)) (`self.Speed`)) (`self.K2_GetActorLocation`))))

(fn `UserConstructionScript`
  (`parent.UserConstructionScript`))