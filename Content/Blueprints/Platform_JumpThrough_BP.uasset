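; One-way platform that the player can jump up through and then land on, made by toggling the Cube's response on a custom collision channel.
; The Cube ignores that channel from construction, switches to Block when player 0 enters the Box (0.2s later if entering from below), and reverts on exit.
; A post-block overlap check works around players getting stuck, but sets the Pawn channel to Ignore rather than the custom one.
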(event `self.ReceiveBeginPlay`)

(event `self.Box.OnComponentBeginOverlap`
  (params (OverlappedComponent :type "PrimitiveComponent Object Reference") (OtherActor :type "Actor Object Reference") (OtherComp :type "PrimitiveComponent Object Reference") (OtherBodyIndex :type Integer) (bFromSweep :type Boolean) (SweepResult :type "HitResult Structure (by ref)"))
  (bind _returnvalue (`GameplayStatics.GetPlayerCharacter` 0))
  (bind _box (`self.Box`))
  (bind (_returnvalue_x _returnvalue_y _returnvalue_z) (`KismetMathLibrary.BreakVector` (`SceneComponent.K2_GetComponentLocation` (`self.Cube`))))
  (bind (_returnvalue_x_2 _returnvalue_y_2 _returnvalue_z_2) (`KismetMathLibrary.BreakVector` (`SceneComponent.K2_GetComponentLocation` (`Character.Mesh` _returnvalue))))
  ;[1 1 1] Activate the platform
  (if (== OtherActor _returnvalue)
    (if (< _returnvalue_z_2 _returnvalue_z)
      (`KismetSystemLibrary.Delay` 0.2))
    (`PrimitiveComponent.SetCollisionResponseToChannel` (`self.Cube`) "ECC_GameTraceChannel2" "ECR_Block")
    ;[1 1 1] Debug Collider
    ; Erro: the players stay stuck in the platform, cause the box checker don't indentify in 0.2s the players got out the overlap
    (bind (_outactors _returnvalue_2) (`KismetSystemLibrary.ComponentOverlapActors` _box (`SceneComponent.K2_GetComponentToWorld` _box) (`|MakeArray` "ObjectTypeQuery3" :!type "EObjectTypeQuery Enum") "/Script/Engine.Actor"))
    (if (not _returnvalue_2)
      (`PrimitiveComponent.SetCollisionResponseToChannel` (`self.Cube`) "ECC_Pawn" "ECR_Ignore"))))

(event `self.Box.OnComponentEndOverlap`
  (params (OverlappedComponent :type "PrimitiveComponent Object Reference") (OtherActor :type "Actor Object Reference") (OtherComp :type "PrimitiveComponent Object Reference") (OtherBodyIndex :type Integer))
  ;[1 1 1] Deactivate the platform
  (if (== OtherActor (`GameplayStatics.GetPlayerCharacter` 0))
    (`PrimitiveComponent.SetCollisionResponseToChannel` (`self.Cube`) "ECC_GameTraceChannel2" "ECR_Ignore")))

(fn `UserConstructionScript`
  ;[1 1 1] Start the platform deactivated
  (`PrimitiveComponent.SetCollisionResponseToChannel` (`self.Cube`) "ECC_GameTraceChannel2" "ECR_Ignore"))